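; Player ship for a shooter, moved in the Y-Z plane by axis input.
; Tick offsets location by Direction and Speed without sweep, then lerps the Pivot rotation to tilt with movement.
; Fire spawns a bullet at FirePosition, or two side-offset bullets once upgraded, with a shot sound.
; Overlapping an item consumes it for the upgrade, while an enemy bullet destroys both actors with explosion sound and Niagara effect.
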(event `self.ReceiveBeginPlay`)

(event `self.ReceiveTick`
  (params (DeltaSeconds :type "Float (single-precision)"))
  ; 이동한다.
  (`self.K2_SetActorLocation` (+ (* DeltaSeconds (* (`self.Direction`) (`self.Speed`))) (`self.K2_GetActorLocation`)))
  (`self.MoveAnimation`))

(event `InputAxis|Horizontal`
  (params (AxisValue :type "Float (single-precision)"))
  ; 방향구하기
  (set `self.Direction` (`KismetMathLibrary.MakeVector` 0.0 AxisValue (stale `InputAxis|Vertical` AxisValue)) :!label _label))

(event `InputAxis|Vertical`
  (params (AxisValue :type "Float (single-precision)"))
  ; 방향구하기
  (goto _label))

(event `InputAction|Fire`
  (params (Key :type "Key Structure"))
  (:`Pressed`
    (`self.FireBullet`)
    (`GameplayStatics.PlaySound2D` "/Game/Sounds/Shoot2.Shoot2" 1.0 1.0 0.0 null null)))

(event `self.Collision.OnComponentBeginOverlap`
  (params (OverlappedComponent :type "PrimitiveComponent Object Reference") (OtherActor :type "Actor Object Reference") (OtherComp :type "PrimitiveComponent Object Reference") (OtherBodyIndex :type Integer) (bFromSweep :type Boolean) (SweepResult :type "HitResult Structure (by ref)"))
  (bind _asbp_item (cast `/Game/Blueprints/BP_Item` OtherActor)
    (:`then`
      (`self.K2_DestroyActor` _asbp_item)
      (set `self.Is Upgrade` true))
    (:`CastFailed`
      (cast `/Game/Blueprints/BP_EnemyBullet` OtherActor)
      (`GameplayStatics.SpawnSound2D` "/Game/Sounds/Explosion.Explosion" 1.0 1.0 0.0 null)
      (`NiagaraFunctionLibrary.SpawnSystemAtLocation` "/Game/Fire_EXP_Vol01_Free/Niagara/EXP/NS_Sub_EXP_Large_001_01.NS_Sub_EXP_Large_001_01" (`self.K2_GetActorLocation`) (struct :`Pitch` 90.0) (1.5 1.5 1.5) true true "AutoRelease")
      (`self.K2_DestroyActor`)
      (`self.K2_DestroyActor` OtherActor))))

(fn `FireBullet`
  (bind _returnvalue (`SceneComponent.K2_GetComponentLocation` (`self.FirePosition`)))
  (if (`self.Is Upgrade`)
    (`|SpawnActorFromClass` "/Game/Blueprints/BP_Bullet.BP_Bullet_C" (`KismetMathLibrary.MakeTransform` (+ _returnvalue (0.0 -80.0 0.0))) "AlwaysSpawn" "MultiplyWithRoot" null null)
    (`|SpawnActorFromClass` "/Game/Blueprints/BP_Bullet.BP_Bullet_C" (`KismetMathLibrary.MakeTransform` (+ _returnvalue (0.0 80.0 0.0))) "AlwaysSpawn" "MultiplyWithRoot" null null)
    (else
      (`|SpawnActorFromClass` "/Game/Blueprints/BP_Bullet.BP_Bullet_C" (`KismetMathLibrary.MakeTransform` (`SceneComponent.K2_GetComponentLocation` (`self.FirePosition`))) "AlwaysSpawn" "MultiplyWithRoot" null null))))

(fn `MoveAnimation`
  (bind (_direction_x _direction_y _direction_z) (`KismetMathLibrary.BreakVector` (`self.Direction`)))
  (bind _pivot (`self.Pivot`))
  (bind (_relativerotation_roll _relativerotation_pitch _relativerotation_yaw) (`KismetMathLibrary.BreakRotator` (`SceneComponent.RelativeRotation` _pivot)))
  (`SceneComponent.K2_SetRelativeRotation` _pivot (`KismetMathLibrary.MakeRotator` 0.0 (`KismetMathLibrary.Lerp` _relativerotation_pitch (* _direction_z -5.0) 0.1) (`KismetMathLibrary.Lerp` _relativerotation_yaw (* _direction_y -45.0) 0.1)) false false))

(fn `UserConstructionScript`)