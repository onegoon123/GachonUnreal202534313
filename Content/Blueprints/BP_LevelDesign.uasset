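; BP_LevelDesign scripts the level's sequence of timed enemy waves followed by a boss encounter.
; On BeginPlay it plays BGM2 and runs a chain of delays, calling Spawn4 to place four BP_Enemy actors at its spawn points with HP that rises over the waves.
; After the last wave it fades the music out, fades in BGM1, then spawns a rotated BP_Boss at SpawnPoint2.
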(event `self.ReceiveBeginPlay`
  (bind _returnvalue (`GameplayStatics.CreateSound2D` "/Game/Sounds/BGM2.BGM2" 1.0 1.0 0.0 null))
  (`AudioComponent.Play` _returnvalue 0.0)
  (set `self.BGM` _returnvalue)
  (`self.Spawn4` 1)
  (`KismetSystemLibrary.Delay` 5.0)
  (`self.Spawn4` 1)
  (`KismetSystemLibrary.Delay` 5.0)
  (`self.Spawn4` 2)
  (`KismetSystemLibrary.Delay` 5.0)
  (`self.Spawn4` 3)
  (`KismetSystemLibrary.Delay` 5.0)
  (`self.Spawn4` 4)
  (`KismetSystemLibrary.Delay` 5.0)
  (`AudioComponent.FadeOut` (`self.BGM`) 3.0 0.0 "Linear")
  (`KismetSystemLibrary.Delay` 3.0)
  (bind _returnvalue_2 (`GameplayStatics.CreateSound2D` "/Game/Sounds/BGM1.BGM1" 1.0 1.0 0.0 null))
  (`AudioComponent.FadeIn` _returnvalue_2 3.0 1.0 0.0 "Linear")
  (bind _returnvalue_3 (`|SpawnActorFromClass` "/Game/Blueprints/BP_Boss.BP_Boss_C" (`SceneComponent.K2_GetComponentToWorld` (`self.SpawnPoint2`)) "Undefined" "MultiplyWithRoot" null null))
  (`self.K2_AddActorWorldRotation` _returnvalue_3 (struct :`Pitch` -90.0 :`Yaw` -89.99) false false))

(fn `Spawn4`
  (params (HP :type Integer))
  (bind _returnvalue (`|SpawnActorFromClass` "/Game/Blueprints/BP_Enemy.BP_Enemy_C" (`SceneComponent.K2_GetComponentToWorld` (`self.SpawnPoint2`)) "Undefined" "MultiplyWithRoot" null null))
  (`/Game/Blueprints/BP_Enemy.SetHP` _returnvalue HP)
  (bind _returnvalue_2 (`|SpawnActorFromClass` "/Game/Blueprints/BP_Enemy.BP_Enemy_C" (`SceneComponent.K2_GetComponentToWorld` (`self.SpawnPoint4`)) "Undefined" "MultiplyWithRoot" null null))
  (`/Game/Blueprints/BP_Enemy.SetHP` _returnvalue_2 HP)
  (bind _returnvalue_3 (`|SpawnActorFromClass` "/Game/Blueprints/BP_Enemy.BP_Enemy_C" (`SceneComponent.K2_GetComponentToWorld` (`self.SpawnPoint3`)) "Undefined" "MultiplyWithRoot" null null))
  (`/Game/Blueprints/BP_Enemy.SetHP` _returnvalue_3 HP)
  (bind _returnvalue_4 (`|SpawnActorFromClass` "/Game/Blueprints/BP_Enemy.BP_Enemy_C" (`SceneComponent.K2_GetComponentToWorld` (`self.SpawnPoint1`)) "Undefined" "MultiplyWithRoot" null null))
  (`/Game/Blueprints/BP_Enemy.SetHP` _returnvalue_4 HP))

(fn `UserConstructionScript`)